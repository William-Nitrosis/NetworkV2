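; BP_WeaponBase is a weapon base Blueprint that orients its skeletal mesh every Tick, with a ThirdPersonGun flag selecting the behavior.
; When the flag is set, the mesh keeps its world yaw and has pitch and roll zeroed.
; Otherwise it follows the player 0 camera, mapping negated camera pitch to roll and offsetting yaw a quarter turn to suit the mesh's sideways orientation.
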(event EventTick
  (params (DeltaSeconds :type Float%20%28single-precision%29))
  (bind _returnvalue (Game|GetPlayerCameraManager 0))
  (bind _skeletalmesh (Variables|Default|GetSkeletalMesh))
  (bind _returnvalue_2 (Camera|GetCameraRotation _returnvalue))
  (if (Variables|Default|GetbThirdPersonGun)
    (Transformation|SetWorldRotation _skeletalmesh (Math|Rotator|MakeRotator 0.0 0.0 (.yaw (Transformation|GetWorldRotation _skeletalmesh))) false false)
    (else
      (Transformation|SetWorldRotation (Variables|Default|GetSkeletalMesh) (Math|Rotator|MakeRotator (* (.pitch _returnvalue_2) -1.0) 0.0 (- (.yaw _returnvalue_2) 9e+01)) false false))))

(fn ConstructionScript)